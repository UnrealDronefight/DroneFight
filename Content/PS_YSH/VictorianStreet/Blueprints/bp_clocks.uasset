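; Placeable street clock prop with two pairs of hands on opposite faces, posed to show a configurable time.
; The construction script picks one of two meshes from ClockType and repositions both hand pairs to fit it.
; It converts between total seconds and hours, minutes and seconds, depending on SetClockByTotalTime, then rolls the hands from the total.
; The event graph is empty, so the clock does not advance during play.
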(fn `UserConstructionScript`
  (bind _total_time (`self.Total Time`))
  (bind _clock_minute_hand (`self.clock_minute_hand`))
  (bind _clock_minute_hand_2 (`self.clock_minute_hand_2`))
  (bind _clock_hourhand_2 (`self.clock_hourhand_2`))
  (bind _staticmeshcomponent (`self.StaticMeshComponent`))
  (bind _clock_hour_hand (`self.clock_hour_hand`))
  (bind (_remainder _returnvalue) (`KismetMathLibrary.FMod` (`KismetMathLibrary.Conv_IntToDouble` (`self.Total Time`)) 60.0))
  (bind _returnvalue_2 (* (`KismetMathLibrary.Conv_IntToDouble` _total_time) (/ 360.0 -43200.0)))
  (bind _returnvalue_3 (* (`KismetMathLibrary.Conv_IntToDouble` _total_time) -0.1))
  ;[1 1 1] Select clock type
  (switch `int` (`self.Clock Type`)
    (:`Default`
      (`StaticMeshComponent.SetStaticMesh` _staticmeshcomponent "/Game/PS_YSH/VictorianStreet/Meshes/Static/sm_clock_a.sm_clock_a" :!label _label)
      ;[1 1 1] Position the clock hands
      (`SceneComponent.K2_SetRelativeLocation` _clock_minute_hand (16.5 -170.0 -52.026001) false false)
      (`SceneComponent.K2_SetRelativeLocation` _clock_hour_hand (16.0 -170.0 -52.026001) false false)
      (`SceneComponent.K2_SetRelativeLocation` _clock_minute_hand_2 (-16.5 -170.0 -52.026001) false false)
      (`SceneComponent.K2_SetRelativeLocation` _clock_hourhand_2 (-16.0 -170.0 -52.026001) false false))
    (:`0`
      (goto _label))
    (:`1`
      (`StaticMeshComponent.SetStaticMesh` _staticmeshcomponent "/Game/PS_YSH/VictorianStreet/Meshes/Static/sm_clock_b.sm_clock_b")
      (`SceneComponent.K2_SetRelativeLocation` _clock_minute_hand (13.5 -118.976997 -129.011993) false false)
      (`SceneComponent.K2_SetRelativeLocation` _clock_hour_hand (13.0 -118.976997 -129.011993) false false)
      (`SceneComponent.K2_SetRelativeLocation` _clock_minute_hand_2 (-13.5 -118.976997 -129.011993) false false)
      (`SceneComponent.K2_SetRelativeLocation` _clock_hourhand_2 (-13.0 -118.976997 -129.011993) false false)))
  (`|ExecutionSequence`
    (:`then_0`
      ;[1 1 1] Set the time
      (if (`self.Set Clock by Total Time?`)
        (set `self.Minutes` (mod _returnvalue 60))
        (set `self.Seconds` (`KismetMathLibrary.FTrunc` _remainder))
        (set `self.Hours` (`.ReturnValue` (`KismetMathLibrary.FMod` (`KismetMathLibrary.Conv_IntToDouble` _returnvalue) 60.0)))
        (else
          (set `self.Total Time` (+ (+ (`self.Seconds`) (* (`self.Minutes`) 60)) (* (`self.Hours`) 3600))))))
    (:`then_1`
      ;[1 1 1] Rotate the clock hands to match the time
      (`SceneComponent.K2_SetRelativeRotation` (`self.clock_minute_hand`) (`KismetMathLibrary.MakeRotator` _returnvalue_3) false false)
      (`SceneComponent.K2_SetRelativeRotation` (`self.clock_minute_hand_2`) (`KismetMathLibrary.MakeRotator` _returnvalue_3 0.0 180.0) false false)
      (`SceneComponent.K2_SetRelativeRotation` (`self.clock_hour_hand`) (`KismetMathLibrary.MakeRotator` _returnvalue_2) false false)
      (`SceneComponent.K2_SetRelativeRotation` (`self.clock_hourhand_2`) (`KismetMathLibrary.MakeRotator` _returnvalue_2 0.0 180.0) false false))))