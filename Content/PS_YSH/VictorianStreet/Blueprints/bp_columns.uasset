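; Modular Victorian street facade column that picks its mesh at construction time from storey and style settings.
; The construction script resets material overrides, then sets a column mesh per storey and style, or a light-blocker mesh when flagged.
; An optional wall extension component gets a block or brick material.
; Two ground-level styles apply hue shift and desaturation through dynamic material instances.
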(fn `Set Wall Extension Material`
  (params (`Wall Mesh` :type "StaticMeshComponent Object Reference"))
  (switch `/Game/PS_YSH/VictorianStreet/Blueprints/EnumeratedLists/e_wall_materials` (`self.Wall Extension Style`)
    (:`NewEnumerator1`
      (`PrimitiveComponent.SetMaterialByName` `Wall Mesh` "col_wall" "/Game/PS_YSH/VictorianStreet/Materials/Instances/mi_block_wall_a.mi_block_wall_a"))
    (:`NewEnumerator3`
      (`PrimitiveComponent.SetMaterialByName` `Wall Mesh` "col_wall" "/Game/PS_YSH/VictorianStreet/Materials/Instances/mi_brick_wall_a.mi_brick_wall_a"))
    (:`NewEnumerator0`
      (`PrimitiveComponent.SetMaterialByName` `Wall Mesh` "col_wall" "/Game/PS_YSH/VictorianStreet/Materials/Instances/mi_brick_wall_b.mi_brick_wall_b"))))

(fn `Style 4 Color`
  (bind _staticmeshcomponent (`self.StaticMeshComponent`))
  (bind _slot_a (`self.slot_a`))
  (if (`MeshComponent.IsMaterialSlotNameValid` _staticmeshcomponent _slot_a)
    (bind _returnvalue (`KismetMaterialLibrary.CreateDynamicMaterialInstance` "/Game/PS_YSH/VictorianStreet/Materials/Instances/mi_facade_e_column_lvl0_unique_a.mi_facade_e_column_lvl0_unique_a"))
    (`MaterialInstanceDynamic.SetScalarParameterValue` _returnvalue "Hue Shift" (`self.Hue Shift 1`))
    (`MaterialInstanceDynamic.SetScalarParameterValue` _returnvalue "Desaturation" (`self.Desaturation 1`))
    (`PrimitiveComponent.SetMaterialByName` _staticmeshcomponent _slot_a _returnvalue)))

(fn `Style 5 Color`
  (bind _staticmeshcomponent (`self.StaticMeshComponent`))
  (bind _slot_a (`self.slot_a`))
  (if (`MeshComponent.IsMaterialSlotNameValid` _staticmeshcomponent _slot_a)
    (bind _returnvalue (`KismetMaterialLibrary.CreateDynamicMaterialInstance` "/Game/PS_YSH/VictorianStreet/Materials/Instances/mi_facade_f_column_unique_a.mi_facade_f_column_unique_a"))
    (`MaterialInstanceDynamic.SetScalarParameterValue` _returnvalue "Hue Shift" (`self.Hue Shift 1`))
    (`MaterialInstanceDynamic.SetScalarParameterValue` _returnvalue "Desaturation" (`self.Desaturation 1`))
    (`PrimitiveComponent.SetMaterialByName` _staticmeshcomponent _slot_a _returnvalue)))

(fn `UserConstructionScript`
  (bind _staticmeshcomponent (`self.StaticMeshComponent`))
  (bind _wall_extension_ (`self.Wall Extension?`))
  (bind _style (`self.Style`))
  (bind _light_blocker_ (`self.Light Blocker?`))
  (bind _staticmeshcomponent_2 (`self.StaticMeshComponent`))
  (bind _staticmeshcomponent_3 (`self.StaticMeshComponent`))
  (bind _staticmeshcomponent_4 (`self.StaticMeshComponent`))
  (bind _light_blocker__2 (`self.Light Blocker?`))
  ;[1 1 1] Reset materials to ensure material overides are reset when switching meshes
  (for (_ _array_index) (`MeshComponent.GetMaterials` _staticmeshcomponent_4)
    (`PrimitiveComponent.SetMaterial` _staticmeshcomponent_4 _array_index null))
  ;[1 1 1] Select storey
  (switch `int` (`self.Storey`)
    (:`0`
      ;[1 1 1] Select mesh (ground level)
      (switch `int` _style
        (:`Default`
          (if _light_blocker__2 :!label _label
            (`StaticMeshComponent.SetStaticMesh` _staticmeshcomponent_3 "/Game/PS_YSH/VictorianStreet/Meshes/Helpers/LightBlockers/sm_blocker_col_600.sm_blocker_col_600" :!label _label_2)
            (else
              (`StaticMeshComponent.SetStaticMesh` _staticmeshcomponent_3 "/Game/PS_YSH/VictorianStreet/Meshes/Static/sm_facade_a_column_lvl0.sm_facade_a_column_lvl0")))
          ;[1 1 1] Add wall extenstion
          (if (`self.Wall Extension?`) :!label _label_3
            (bind _returnvalue (`AddComponent|NODE_AddStaticMeshComponent-8`))
            ;[1 1 1] Set wall extension material
            (`self.Set Wall Extension Material` _returnvalue) ; Set wall extension material
          ))
        (:`0`
          (goto _label))
        (:`1`
          (if _light_blocker__2
            (goto _label_2)
            (else
              (`StaticMeshComponent.SetStaticMesh` _staticmeshcomponent_3 "/Game/PS_YSH/VictorianStreet/Meshes/Static/sm_facade_b_column_lvl0.sm_facade_b_column_lvl0")
              (goto _label_3))))
        (:`2`
          (if _light_blocker_
            (`StaticMeshComponent.SetStaticMesh` _staticmeshcomponent_3 "/Game/PS_YSH/VictorianStreet/Meshes/Helpers/LightBlockers/sm_blocker_col_450.sm_blocker_col_450")
            (else
              (`StaticMeshComponent.SetStaticMesh` _staticmeshcomponent_3 "/Game/PS_YSH/VictorianStreet/Meshes/Static/sm_facade_c_column_lvl0.sm_facade_c_column_lvl0")))
          (if (`self.Wall Extension?`)
            (bind _returnvalue_2 (`AddComponent|NODE_AddStaticMeshComponent-9`))
            (`self.Set Wall Extension Material` _returnvalue_2)))
        (:`3`
          (if _light_blocker__2
            (goto _label_2)
            (else
              (`StaticMeshComponent.SetStaticMesh` _staticmeshcomponent_3 "/Game/PS_YSH/VictorianStreet/Meshes/Static/sm_facade_d_column_lvl0.sm_facade_d_column_lvl0")
              (if (`self.Wall Extension?`)
                (bind _returnvalue_3 (`AddComponent|NODE_AddStaticMeshComponent-11`))
                (`self.Set Wall Extension Material` _returnvalue_3)))))
        (:`4`
          (if _light_blocker_
            (goto _label_2)
            (else
              (`StaticMeshComponent.SetStaticMesh` _staticmeshcomponent_3 "/Game/PS_YSH/VictorianStreet/Meshes/Static/sm_facade_e_column_lvl0.sm_facade_e_column_lvl0")
              ;[1 1 1] Set color options
              (`self.Style 4 Color`)
              (goto _label_3))))
        (:`5`
          (if _light_blocker_
            (goto _label_2)
            (else
              (`StaticMeshComponent.SetStaticMesh` _staticmeshcomponent_3 "/Game/PS_YSH/VictorianStreet/Meshes/Static/sm_facade_f_column_lvl0.sm_facade_f_column_lvl0")
              (`self.Style 5 Color`)
              (goto _label_3))))))
    (:`1`
      ;[1 1 1] Select mesh (first storey)
      (if (`self.Light Blocker?`)
        (`StaticMeshComponent.SetStaticMesh` _staticmeshcomponent_2 "/Game/PS_YSH/VictorianStreet/Meshes/Helpers/LightBlockers/sm_blocker_col_400.sm_blocker_col_400")
        (else
          (switch `int` _style
            (:`Default`
              (`StaticMeshComponent.SetStaticMesh` _staticmeshcomponent_2 "/Game/PS_YSH/VictorianStreet/Meshes/Static/sm_facade_c_column_lvl1.sm_facade_c_column_lvl1" :!label _label_4))
            (:`0`
              (`StaticMeshComponent.SetStaticMesh` _staticmeshcomponent_2 "/Game/PS_YSH/VictorianStreet/Meshes/Static/sm_facade_a_column_lvl1.sm_facade_a_column_lvl1"))
            (:`1`
              (`StaticMeshComponent.SetStaticMesh` _staticmeshcomponent_2 "/Game/PS_YSH/VictorianStreet/Meshes/Static/sm_facade_b_column_lvl1.sm_facade_b_column_lvl1"))
            (:`2`
              (goto _label_4)))))
      (if _wall_extension_ :!label _label_5
        (bind _returnvalue_4 (`AddComponent|NODE_AddStaticMeshComponent-10`))
        (`self.Set Wall Extension Material` _returnvalue_4)))
    (:`2`
      ;[1 1 1] Slect mesh (second storey +)
      (if (`self.Light Blocker?`)
        (`StaticMeshComponent.SetStaticMesh` _staticmeshcomponent "/Game/PS_YSH/VictorianStreet/Meshes/Helpers/LightBlockers/sm_blocker_col_400.sm_blocker_col_400")
        (goto _label_5)
        (else
          (switch `int` _style
            (:`Default`
              (`StaticMeshComponent.SetStaticMesh` _staticmeshcomponent "/Game/PS_YSH/VictorianStreet/Meshes/Static/sm_facade_c_column_lvl2.sm_facade_c_column_lvl2" :!label _label_6)
              (goto _label_5))
            (:`0`
              (`StaticMeshComponent.SetStaticMesh` _staticmeshcomponent "/Game/PS_YSH/VictorianStreet/Meshes/Static/sm_facade_a_column_lvl2.sm_facade_a_column_lvl2")
              (if _wall_extension_
                (bind _returnvalue_5 (`AddComponent|NODE_AddStaticMeshComponent-12`))
                (`self.Set Wall Extension Material` _returnvalue_5)))
            (:`1`
              (`StaticMeshComponent.SetStaticMesh` _staticmeshcomponent "/Game/PS_YSH/VictorianStreet/Meshes/Static/sm_facade_b_column_lvl2.sm_facade_b_column_lvl2")
              (goto _label_5))
            (:`2`
              (goto _label_6))))))))