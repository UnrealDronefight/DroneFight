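; Chimney pipe prop for the Victorian street that randomises its look and can emit wind-blown smoke.
; The construction script uses seeded streams to pick one of two meshes, rotate it (quarter turns or free yaw by type), vary its height and desaturate it through a dynamic material instance.
; It also toggles smoke auto-activation and sets particle direction from an assigned actor's forward vector times a wind strength multiplier.
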(fn `UserConstructionScript`
  (bind _staticmeshcomponent (`self.StaticMeshComponent`))
  (bind _wind_directional_actor (`self.Wind Directional Actor`))
  (bind _slot_a (`self.slot_a`))
  ;[1 1 1] Ensure the BP is updated with latest settings
  (if (`self.Refresh?`)
    _
    (else
      _))
  (set `self.Refresh?` false)
  (`|ExecutionSequence`
    (:`then_0`
      ;[1 1 1] Random selection between two types of pipe
      (switch `int` (`KismetMathLibrary.RandomIntegerInRangeFromStream` (`self.Pipe Type Seed`) 0 1)
        (:`Default`
          (`StaticMeshComponent.SetStaticMesh` _staticmeshcomponent "/Game/PS_YSH/VictorianStreet/Meshes/Static/sm_chimney_pipe_a.sm_chimney_pipe_a" :!label _label)
          ;[1 1 1] Random orientation
          (switch `int` (`KismetMathLibrary.RandomIntegerInRangeFromStream` (`self.Rotation Seed A`) 0 3)
            (:`Default`
              (`SceneComponent.K2_SetWorldRotation` :`self` _staticmeshcomponent :!label _label_2))
            (:`0`
              (goto _label_2))
            (:`1`
              (`SceneComponent.K2_SetWorldRotation` _staticmeshcomponent (struct :`Yaw` 90.0) false false))
            (:`2`
              (`SceneComponent.K2_SetWorldRotation` _staticmeshcomponent (struct :`Yaw` 180.0) false false))
            (:`3`
              (`SceneComponent.K2_SetWorldRotation` _staticmeshcomponent (struct :`Yaw` 270.0) false false))))
        (:`0`
          (goto _label))
        (:`1`
          (`StaticMeshComponent.SetStaticMesh` _staticmeshcomponent "/Game/PS_YSH/VictorianStreet/Meshes/Static/sm_chimney_pipe_b.sm_chimney_pipe_b")
          (`SceneComponent.K2_SetWorldRotation` _staticmeshcomponent (`KismetMathLibrary.MakeRotator` 0.0 0.0 (`KismetMathLibrary.RandomFloatInRangeFromStream` (`self.Rotation Seed B`) 0.0 359.9)) false false)))
      ;[1 1 1] Random scale
      (`SceneComponent.SetWorldScale3D` _staticmeshcomponent (`KismetMathLibrary.MakeVector` 1.0 1.0 (`KismetMathLibrary.RandomFloatInRangeFromStream` (`self.Scale Seed A`) (`self.Scale Min`) (`self.Scale Max`))))
      ;[1 1 1] Random desaturation
      (if (`MeshComponent.IsMaterialSlotNameValid` _staticmeshcomponent _slot_a)
        (bind _returnvalue (`KismetMaterialLibrary.CreateDynamicMaterialInstance` "/Game/PS_YSH/VictorianStreet/Materials/Instances/mi_chimney_pipes.mi_chimney_pipes"))
        (`MaterialInstanceDynamic.SetScalarParameterValue` _returnvalue "Desaturation" (`KismetMathLibrary.RandomFloatInRangeFromStream` (`self.Desturation Seed`) (`self.Desaturation Min`) (`self.Desaturation Max`)))
        (`PrimitiveComponent.SetMaterialByName` _staticmeshcomponent _slot_a _returnvalue)))
    (:`then_1`
      ;[1 1 1] Enable smoke that blows according to the wind direction
      (`ActorComponent.SetAutoActivate` (`self.p_smoke`) (`self.Enable Smoke?`))
      (`/Engine/EditorBlueprintResources/StandardMacros.IsValid` _wind_directional_actor ; Has a directional light been assigned?
        (:`Is Valid`
          (`ParticleSystemComponent.SetVectorParameter` (`self.p_smoke`) "Direction" (* (`KismetMathLibrary.Conv_RotatorToVector` (`self.K2_GetActorRotation` _wind_directional_actor)) (`self.Wind Stength Multiplier`))))))))