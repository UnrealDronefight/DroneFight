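; Configurable chimney prop for the Victorian street set, assembled entirely in the construction script.
; A ChimneyType enum picks the short, mid or long chimney mesh for the static mesh component.
; A WallMaterial enum then sets material slot 0 to block or one of two brick wall materials.
; The event graph holds only disabled placeholder events, so there is no runtime logic.
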(fn `UserConstructionScript`
  (bind _staticmeshcomponent (`self.StaticMeshComponent`))
  (bind _staticmeshcomponent_2 (`self.StaticMeshComponent`))
  (`|ExecutionSequence`
    (:`then_0`
      ;[1 1 1] Select the chimney type
      (switch `/Game/PS_YSH/VictorianStreet/Blueprints/EnumeratedLists/e_chimney_type` (`self.Chimney Type`)
        (:`NewEnumerator1`
          (`StaticMeshComponent.SetStaticMesh` _staticmeshcomponent "/Game/PS_YSH/VictorianStreet/Meshes/Static/sm_chimney_a_short.sm_chimney_a_short"))
        (:`NewEnumerator0`
          (`StaticMeshComponent.SetStaticMesh` _staticmeshcomponent "/Game/PS_YSH/VictorianStreet/Meshes/Static/sm_chimney_a_mid.sm_chimney_a_mid"))
        (:`NewEnumerator2`
          (`StaticMeshComponent.SetStaticMesh` _staticmeshcomponent "/Game/PS_YSH/VictorianStreet/Meshes/Static/sm_chimney_a_long.sm_chimney_a_long"))))
    (:`then_1`
      ;[1 1 1] Select the wall material
      (switch `/Game/PS_YSH/VictorianStreet/Blueprints/EnumeratedLists/e_wall_materials` (`self.Wall Material`)
        (:`NewEnumerator1`
          (`PrimitiveComponent.SetMaterial` _staticmeshcomponent_2 0 "/Game/PS_YSH/VictorianStreet/Materials/Instances/mi_block_wall_a.mi_block_wall_a"))
        (:`NewEnumerator3`
          (`PrimitiveComponent.SetMaterial` _staticmeshcomponent_2 0 "/Game/PS_YSH/VictorianStreet/Materials/Instances/mi_brick_wall_a.mi_brick_wall_a"))
        (:`NewEnumerator0`
          (`PrimitiveComponent.SetMaterial` _staticmeshcomponent_2 0 "/Game/PS_YSH/VictorianStreet/Materials/Instances/mi_brick_wall_b.mi_brick_wall_b"))))))