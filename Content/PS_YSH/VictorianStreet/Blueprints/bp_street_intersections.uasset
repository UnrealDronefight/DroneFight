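; Construction-script Blueprint for placing Victorian street intersection pieces.
; An IntersectionStyle option selects the static mesh for a 3-way, skewed 3-way or 4-way junction.
; A Mirror flag flips the mesh by setting a negative Y world scale, otherwise resetting it to unit scale.
; The event graph holds only disabled stub events, so it has no runtime logic.
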(fn `UserConstructionScript`
  (bind _staticmeshcomponent (`self.StaticMeshComponent`))
  (bind _staticmeshcomponent_2 (`self.StaticMeshComponent`))
  ;[1 1 1] Mirror mesh?
  (if (`self.Mirror?`)
    (`SceneComponent.SetWorldScale3D` _staticmeshcomponent_2 (1.0 -1.0 1.0))
    (else
      (`SceneComponent.SetWorldScale3D` _staticmeshcomponent_2 (1.0 1.0 1.0))))
  ;[1 1 1] Select mesh
  (switch `/Game/PS_YSH/VictorianStreet/Blueprints/EnumeratedLists/e_intersections` (`self.Intersection Style`)
    (:`NewEnumerator1`
      (`StaticMeshComponent.SetStaticMesh` _staticmeshcomponent "/Game/PS_YSH/VictorianStreet/Meshes/Static/sm_intersection_90deg_a.sm_intersection_90deg_a"))
    (:`NewEnumerator0`
      (`StaticMeshComponent.SetStaticMesh` _staticmeshcomponent "/Game/PS_YSH/VictorianStreet/Meshes/Static/sm_intersection_10deg_a.sm_intersection_10deg_a"))
    (:`NewEnumerator2`
      (`StaticMeshComponent.SetStaticMesh` _staticmeshcomponent "/Game/PS_YSH/VictorianStreet/Meshes/Static/sm_intersection_90deg_b.sm_intersection_90deg_b"))))