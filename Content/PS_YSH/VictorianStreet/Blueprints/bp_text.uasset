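; Victorian street signage Blueprint that places a selectable shop text or divider as either a decal or a mesh decal.
; The construction script adds a decal or static mesh component based on TrueDecal, then creates a dynamic material instance for color, dirt and wear settings.
; SetText maps the Text choice to a sub-UV frame in the material.
; The mesh variant also feeds its forward vector and a multiplier into world position offset.
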(fn `Set Text`
  (switch `/Game/PS_YSH/VictorianStreet/Blueprints/EnumeratedLists/e_text_options` (`self.Text`)
    (:`NewEnumerator0`
      (set `self.Sub UV Integer` 5))
    (:`NewEnumerator1`
      (set `self.Sub UV Integer` 45))
    (:`NewEnumerator2`
      (set `self.Sub UV Integer` 0))
    (:`NewEnumerator3`
      (set `self.Sub UV Integer` 6))
    (:`NewEnumerator4`
      (set `self.Sub UV Integer` 12))
    (:`NewEnumerator5`
      (set `self.Sub UV Integer` 56))
    (:`NewEnumerator6`
      (set `self.Sub UV Integer` 19))
    (:`NewEnumerator7`
      (set `self.Sub UV Integer` 29))
    (:`NewEnumerator8`
      (set `self.Sub UV Integer` 53))
    (:`NewEnumerator9`
      (set `self.Sub UV Integer` 15))
    (:`NewEnumerator10`
      (set `self.Sub UV Integer` 54))
    (:`NewEnumerator11`
      (set `self.Sub UV Integer` 44))
    (:`NewEnumerator12`
      (set `self.Sub UV Integer` 47))
    (:`NewEnumerator13`
      (set `self.Sub UV Integer` 32))
    (:`NewEnumerator14`
      (set `self.Sub UV Integer` 41))
    (:`NewEnumerator15`
      (set `self.Sub UV Integer` 3))
    (:`NewEnumerator16`
      (set `self.Sub UV Integer` 13))
    (:`NewEnumerator17`
      (set `self.Sub UV Integer` 9))
    (:`NewEnumerator18`
      (set `self.Sub UV Integer` 16))
    (:`NewEnumerator19`
      (set `self.Sub UV Integer` 30))
    (:`NewEnumerator20`
      (set `self.Sub UV Integer` 52))
    (:`NewEnumerator21`
      (set `self.Sub UV Integer` 38))
    (:`NewEnumerator22`
      (set `self.Sub UV Integer` 37))
    (:`NewEnumerator23`
      (set `self.Sub UV Integer` 10))
    (:`NewEnumerator24`
      (set `self.Sub UV Integer` 40))
    (:`NewEnumerator25`
      (set `self.Sub UV Integer` 48))
    (:`NewEnumerator26`
      (set `self.Sub UV Integer` 20))
    (:`NewEnumerator27`
      (set `self.Sub UV Integer` 1))
    (:`NewEnumerator28`
      (set `self.Sub UV Integer` 2))
    (:`NewEnumerator29`
      (set `self.Sub UV Integer` 49))
    (:`NewEnumerator30`
      (set `self.Sub UV Integer` 51))
    (:`NewEnumerator31`
      (set `self.Sub UV Integer` 17))
    (:`NewEnumerator32`
      (set `self.Sub UV Integer` 39))
    (:`NewEnumerator33`
      (set `self.Sub UV Integer` 31))
    (:`NewEnumerator34`
      (set `self.Sub UV Integer` 50))
    (:`NewEnumerator35`
      (set `self.Sub UV Integer` 28))
    (:`NewEnumerator36`
      (set `self.Sub UV Integer` 8))
    (:`NewEnumerator37`
      (set `self.Sub UV Integer` 4))
    (:`NewEnumerator38`
      (set `self.Sub UV Integer` 43))
    (:`NewEnumerator39`
      (set `self.Sub UV Integer` 33))
    (:`NewEnumerator40`
      (set `self.Sub UV Integer` 25))
    (:`NewEnumerator41`
      (set `self.Sub UV Integer` 24))
    (:`NewEnumerator42`
      (set `self.Sub UV Integer` 26))
    (:`NewEnumerator43`
      (set `self.Sub UV Integer` 57))
    (:`NewEnumerator44`
      (set `self.Sub UV Integer` 22))
    (:`NewEnumerator45`
      (set `self.Sub UV Integer` 21))
    (:`NewEnumerator46`
      (set `self.Sub UV Integer` 55))
    (:`NewEnumerator47`
      (set `self.Sub UV Integer` 14))
    (:`NewEnumerator48`
      (set `self.Sub UV Integer` 11))
    (:`NewEnumerator49`
      (set `self.Sub UV Integer` 34))
    (:`NewEnumerator50`
      (set `self.Sub UV Integer` 7))
    (:`NewEnumerator51`
      (set `self.Sub UV Integer` 27))
    (:`NewEnumerator52`
      (set `self.Sub UV Integer` 46))
    (:`NewEnumerator53`
      (set `self.Sub UV Integer` 36))
    (:`NewEnumerator54`
      (set `self.Sub UV Integer` 42))
    (:`NewEnumerator55`
      (set `self.Sub UV Integer` 23))
    (:`NewEnumerator56`
      (set `self.Sub UV Integer` 35))
    (:`NewEnumerator57`
      (set `self.Sub UV Integer` 18))
    (:`NewEnumerator58`
      (set `self.Sub UV Integer` 58))
    (:`NewEnumerator59`
      (set `self.Sub UV Integer` 59))
    (:`NewEnumerator60`
      (set `self.Sub UV Integer` 60))
    (:`NewEnumerator61`
      (set `self.Sub UV Integer` 61))
    (:`NewEnumerator62`
      (set `self.Sub UV Integer` 62))
    (:`NewEnumerator63`
      (set `self.Sub UV Integer` 63))))

(fn `UserConstructionScript`
  (bind _returnvalue (`KismetMathLibrary.Conv_IntToDouble` (`self.Sub UV Integer`)))
  ;[1 1 1] Select type of decal
  (if (`self.True Decal?`)
    (bind _returnvalue_2 (`AddComponent|NODE_AddDecalComponent-0` :`RelativeTransform` (`KismetMathLibrary.MakeTransform` (0.0 0.0 0.0) (struct :`Pitch` 180.0 :`Roll` -90.0) (1.0 1.0 2.0))))
    (bind _returnvalue_3 (`DecalComponent.CreateDynamicMaterialInstance` _returnvalue_2))
    ;[1 1 1] Select the text
    (`self.Set Text`)
    ;[1 1 1] Select approriate subUV
    (`MaterialInstanceDynamic.SetScalarParameterValue` _returnvalue_3 "Sub UV Frame" _returnvalue)
    ;[1 1 1] Set color, dirt, and wear options
    (`MaterialInstanceDynamic.SetVectorParameterValue` _returnvalue_3 "BaseColorTint" (`self.Color`))
    (`MaterialInstanceDynamic.SetScalarParameterValue` _returnvalue_3 "Colorize" (`self.Colorize`))
    (`MaterialInstanceDynamic.SetVectorParameterValue` _returnvalue_3 "Wear - Base Color Tint" (`self.Dirt - Color Tint`))
    (`MaterialInstanceDynamic.SetScalarParameterValue` _returnvalue_3 "Wear - Desaturate" (`self.Dirt - Desaturate`))
    (`MaterialInstanceDynamic.SetScalarParameterValue` _returnvalue_3 "New Black Value" (`self.Dirt Black Value`))
    (`MaterialInstanceDynamic.SetScalarParameterValue` _returnvalue_3 "New Middle Value" (`self.Dirt Middle Value`))
    (`MaterialInstanceDynamic.SetScalarParameterValue` _returnvalue_3 "New White Value" (`self.Dirt White Value`))
    (`MaterialInstanceDynamic.SetScalarParameterValue` _returnvalue_3 "Wear New Black Value" (`self.Wear Black Value`))
    (`MaterialInstanceDynamic.SetScalarParameterValue` _returnvalue_3 "Wear New Middle Value" (`self.Wear Middle Value`))
    (`MaterialInstanceDynamic.SetScalarParameterValue` _returnvalue_3 "Wear New White Value" (`self.Wear White Value`))
    (else
      (bind _returnvalue_4 (`AddComponent|NODE_AddStaticMeshComponent-0`))
      (bind _returnvalue_5 (`KismetMaterialLibrary.CreateDynamicMaterialInstance` "/Game/PS_YSH/VictorianStreet/Materials/Instances/mi_text_decalmesh.mi_text_decalmesh"))
      (`self.Set Text`)
      (`MaterialInstanceDynamic.SetScalarParameterValue` _returnvalue_5 "Sub UV Frame" _returnvalue)
      ;[1 1 1] Set WPO orientation
      (`MaterialInstanceDynamic.SetVectorParameterValue` _returnvalue_5 "WPO" (`KismetMathLibrary.Conv_VectorToLinearColor` (`SceneComponent.GetForwardVector` _returnvalue_4)))
      (`MaterialInstanceDynamic.SetScalarParameterValue` _returnvalue_5 "WPO Multiplier" (`self.WPO Multiplier`))
      (`MaterialInstanceDynamic.SetVectorParameterValue` _returnvalue_5 "BaseColorTint" (`self.Color`))
      (`MaterialInstanceDynamic.SetScalarParameterValue` _returnvalue_5 "Colorize" (`self.Colorize`))
      (`MaterialInstanceDynamic.SetVectorParameterValue` _returnvalue_5 "Wear - Base Color Tint" (`self.Dirt - Color Tint`))
      (`MaterialInstanceDynamic.SetScalarParameterValue` _returnvalue_5 "Wear - Desaturate" (`self.Dirt - Desaturate`))
      (`MaterialInstanceDynamic.SetScalarParameterValue` _returnvalue_5 "New Black Value" (`self.Dirt Black Value`))
      (`MaterialInstanceDynamic.SetScalarParameterValue` _returnvalue_5 "New Middle Value" (`self.Dirt Middle Value`))
      (`MaterialInstanceDynamic.SetScalarParameterValue` _returnvalue_5 "New White Value" (`self.Dirt White Value`))
      (`MaterialInstanceDynamic.SetScalarParameterValue` _returnvalue_5 "Wear New Black Value" (`self.Wear Black Value`))
      (`MaterialInstanceDynamic.SetScalarParameterValue` _returnvalue_5 "Wear New Middle Value" (`self.Wear Middle Value`))
      (`MaterialInstanceDynamic.SetScalarParameterValue` _returnvalue_5 "Wear New White Value" (`self.Wear White Value`))
      (`PrimitiveComponent.SetMaterial` _returnvalue_4 0 _returnvalue_5))))