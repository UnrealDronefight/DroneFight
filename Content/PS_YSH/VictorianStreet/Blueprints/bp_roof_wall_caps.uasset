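; Construction-script Blueprint for a roof end wall cap piece in the Victorian Street environment set.
; The RoofStyle option selects one of two roof end meshes for the static mesh component.
; A helper function then applies a block or brick wall material from WallCapStyle to a named material slot, if that slot exists on the mesh.
; The event graph holds no active logic.
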(fn `Set Wall Cap Material`
  (params (Mesh :type "StaticMeshComponent Object Reference"))
  (bind _slot_a (`self.Slot A`))
  ;[1 1 1] Set the wall material
  (if (`MeshComponent.IsMaterialSlotNameValid` Mesh _slot_a)
    (switch `/Game/PS_YSH/VictorianStreet/Blueprints/EnumeratedLists/e_wall_materials` (`self.Wall Cap Style`)
      (:`NewEnumerator1`
        (`PrimitiveComponent.SetMaterialByName` Mesh _slot_a "/Game/PS_YSH/VictorianStreet/Materials/Instances/mi_block_wall_a.mi_block_wall_a"))
      (:`NewEnumerator3`
        (`PrimitiveComponent.SetMaterialByName` Mesh _slot_a "/Game/PS_YSH/VictorianStreet/Materials/Instances/mi_brick_wall_a.mi_brick_wall_a"))
      (:`NewEnumerator0`
        (`PrimitiveComponent.SetMaterialByName` Mesh _slot_a "/Game/PS_YSH/VictorianStreet/Materials/Instances/mi_brick_wall_b.mi_brick_wall_b")))))

(fn `UserConstructionScript`
  (bind _staticmeshcomponent (`self.StaticMeshComponent`))
  ;[1 1 1] Select the roof mesh
  (switch `/Game/PS_YSH/VictorianStreet/Blueprints/EnumeratedLists/e_roof_styles` (`self.Roof Style`)
    (:`NewEnumerator2`
      (`StaticMeshComponent.SetStaticMesh` _staticmeshcomponent "/Game/PS_YSH/VictorianStreet/Meshes/Static/sm_roof_a_end.sm_roof_a_end"))
    (:`NewEnumerator4`
      (`StaticMeshComponent.SetStaticMesh` _staticmeshcomponent "/Game/PS_YSH/VictorianStreet/Meshes/Static/sm_roof_b_end.sm_roof_b_end")))
  (`self.Set Wall Cap Material` _staticmeshcomponent))